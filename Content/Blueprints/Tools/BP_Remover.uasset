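; BP_Remover is a tool that deletes physics objects the player aims at.
; Both fire events, named as multicasts, line trace from the pawn's camera against PhysicsBody objects and play a shoot sound on a hit.
; Primary fire destroys the hit actor alone.
; Alt fire works only on BP_BaseObject hits, destroying everything in its AttachedObjects list before the object itself.
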(event EventMulticastFireWeapon
  (params (OwningPawn :type BP%20Sandbox%20Character%20Object%20Reference) (Pressed :type Boolean) (Scale :type Vector :default "0, 0, 0") (ConstraintInfo :type ST%20Constraint%20Info%20Structure) (Mass%28kg%29 :type Float%20%28single-precision%29) (Thrust%28N%29 :type Float%20%28single-precision%29) (SelectedKey :type Input%20Chord%20Structure))
  (bind _camera (Variables|/Game/Blueprints/BP_SandboxCharacter.BP_SandboxCharacter_C|GetCamera OwningPawn))
  (bind _returnvalue (Transformation|GetWorldLocation _camera))
  (Utilities|IsValid OwningPawn
    (:Is%20Valid
      ;[1 1 1] Check if firing
      (if Pressed
        ;[1 1 1] Trace a line from player's eyes to 1000 cm away
        (bind _outhit (Collision|LineTraceForObjects _returnvalue (+ _returnvalue (* (Math|Vector|GetForwardVector _camera) 1e+04)) (Utilities|Array|MakeArray "ObjectTypeQuery4") false 0 "None"))
        (Utilities|IsValid (.hitactor _outhit)
          (:Is%20Valid
            (Audio|PlaySoundatLocation "/Game/Audio/SC_ToolShoot.SC_ToolShoot" (Transformation|GetActorLocation OwningPawn) "0, 0, 0" 1.0 1.0 0.0 0 0 0)
            (Actor|DestroyActor (.hitactor _outhit))))))))

(event EventMulticastAltFireWeapon
  (params (OwningPawn :type BP%20Sandbox%20Character%20Object%20Reference) (Pressed :type Boolean))
  (bind _camera (Variables|/Game/Blueprints/BP_SandboxCharacter.BP_SandboxCharacter_C|GetCamera OwningPawn))
  (bind _returnvalue (Transformation|GetWorldLocation _camera))
  (if Pressed
    (Utilities|IsValid OwningPawn
      (:Is%20Valid
        ;[1 1 1] Trace a line from player's eyes to 10000 cm away
        (bind _outhit (Collision|LineTraceForObjects _returnvalue (+ _returnvalue (* (Math|Vector|GetForwardVector _camera) 1e+04)) (Utilities|Array|MakeArray "ObjectTypeQuery4") false 0 "None"))
        ;[1 1 1] Give some feedback to the player telling them they hit a valid object
        (Utilities|IsValid (.hitactor _outhit)
          (:Is%20Valid
            (Audio|PlaySoundatLocation "/Game/Audio/SC_ToolShoot.SC_ToolShoot" (Transformation|GetActorLocation OwningPawn) "0, 0, 0" 1.0 1.0 0.0 0 0 0)
            ;[1 1 1] Find all attached objects and delete them before deleting the targeted object
            (bind _asbp_base_object (Utilities|Casting|CastToBP_BaseObject (.hitactor _outhit)))
            (for _array_element (Variables|/Game/Blueprints/BP_BaseObject.BP_BaseObject_C|GetAttachedObjects _asbp_base_object)
              (Actor|DestroyActor _array_element))
            (Actor|DestroyActor (.hitactor _outhit))))))))

(fn ConstructionScript
  (|CallParentFunction))