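; Constraint tool that links two physics objects picked by successive shots, using a physics constraint created at runtime.
; A multicast fire event traces from the pawn's camera for physics bodies, storing the first hit and joining it to the second.
; The constraint takes its angular and linear limits from the passed ConstraintInfo.
; BP_BaseObject actors record each other in AttachedObjects, then the selection clears.
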(event EventMulticastFireWeapon
  (params (OwningPawn :type BP%20Sandbox%20Character%20Object%20Reference) (Pressed :type Boolean) (Scale :type Vector :default "0, 0, 0") (ConstraintInfo :type ST%20Constraint%20Info%20Structure) (Mass%28kg%29 :type Float%20%28single-precision%29) (Thrust%28N%29 :type Float%20%28single-precision%29) (SelectedKey :type Input%20Chord%20Structure))
  (bind (_rotlimits _rotlimittypes _linearlimits _linearlimittypes) (Utilities|Struct|BreakST_ConstraintInfo ConstraintInfo))
  (bind _camera (Variables|/Game/Blueprints/BP_SandboxCharacter.BP_SandboxCharacter_C|GetCamera OwningPawn))
  (bind _returnvalue (Transformation|GetWorldLocation _camera))
  (bind (_x _y _z) (Math|Vector|BreakVector _linearlimits))
  (bind (_x_2 _y_2 _z_2) (Math|Vector|BreakVector _rotlimits))
  (Utilities|IsValid OwningPawn
    (:Is%20Valid
      (if Pressed
        ;[1 1 1] Trace a line from player's eyes to 1000 cm away
        (bind _outhit (Collision|LineTraceForObjects _returnvalue (+ _returnvalue (* (Math|Vector|GetForwardVector _camera) 1e+04)) (Utilities|Array|MakeArray "ObjectTypeQuery4") false 0 "None"))
        (Utilities|IsValid (.hitactor _outhit)
          (:Is%20Valid
            (Audio|PlaySoundatLocation "/Game/Audio/SC_ToolShoot.SC_ToolShoot" (Transformation|GetActorLocation) "0, 0, 0" 1.0 1.0 0.0 0 0 0)
            (if (Variables|Default|GetPickedFirst)
              (bind _output_get (Variables|Default|SetSecondObject (.hitactor _outhit)))
              (Variables|Default|SetPickedFirst false)
              (bind _returnvalue_2 (AddComponent|AddPhysicsConstraintComponent (stale _output_get_2) false (Math|Transform|MakeTransform (Math|Transform|InverseTransformLocation (Transformation|GetWorldTransform (Actor|GetComponentbyClass (stale _output_get_2) "/Script/Engine.PrimitiveComponent")) (Transformation|GetWorldLocation (Actor|GetComponentbyClass _output_get "/Script/Engine.PrimitiveComponent"))) "90.000000,0.000000, 0")))
              (Class|PhysicsConstraintComponent|SetConstrainedComponents _returnvalue_2 (Actor|GetComponentbyClass (stale _output_get_2) "/Script/Engine.PrimitiveComponent") "None" (Actor|GetComponentbyClass _output_get "/Script/Engine.PrimitiveComponent") "None")
              (Utilities|FlowControl|Sequence
                (:then_0
                  ;[1 1 1] Set angular limits for constraint
                  (Class|PhysicsConstraintComponent|SetAngularSwing1Limit _returnvalue_2 (Utilities|Enum|ByteToEnumEAngularConstraintMotion (Math|Conversions|ToByte(Integer) (Utilities|Array|Get(acopy) _rotlimittypes))) _x_2)
                  (Class|PhysicsConstraintComponent|SetAngularSwing2Limit _returnvalue_2 (Utilities|Enum|ByteToEnumEAngularConstraintMotion (Math|Conversions|ToByte(Integer) (Utilities|Array|Get(acopy) _rotlimittypes 1))) _y_2)
                  (Class|PhysicsConstraintComponent|SetAngularTwistLimit _returnvalue_2 (Utilities|Enum|ByteToEnumEAngularConstraintMotion (Math|Conversions|ToByte(Integer) (Utilities|Array|Get(acopy) _rotlimittypes 2))) _z_2))
                (:then_1
                  ;[1 1 1] Set the linear limits
                  (Class|PhysicsConstraintComponent|SetLinearXLimit _returnvalue_2 (Utilities|Enum|ByteToEnumELinearConstraintMotion (Math|Conversions|ToByte(Integer) (Utilities|Array|Get(acopy) _linearlimittypes))) _x)
                  (Class|PhysicsConstraintComponent|SetLinearYLimit _returnvalue_2 (Utilities|Enum|ByteToEnumELinearConstraintMotion (Math|Conversions|ToByte(Integer) (Utilities|Array|Get(acopy) _linearlimittypes 1))) _y)
                  (Class|PhysicsConstraintComponent|SetLinearZLimit _returnvalue_2 (Utilities|Enum|ByteToEnumELinearConstraintMotion (Math|Conversions|ToByte(Integer) (Utilities|Array|Get(acopy) _linearlimittypes 2))) _z))
                (:then_2
                  ;[1 1 1] Add objects to eachother's list of attached objects
                  (bind _asbp_base_object (Utilities|Casting|CastToBP_BaseObject (Variables|Default|GetFirstObject)))
                  (Utilities|Array|Add (Variables|/Game/Blueprints/BP_BaseObject.BP_BaseObject_C|GetAttachedObjects _asbp_base_object) (Variables|Default|GetSecondObject))
                  (bind _asbp_base_object_2 (Utilities|Casting|CastToBP_BaseObject (Variables|Default|GetSecondObject)))
                  (Utilities|Array|Add (Variables|/Game/Blueprints/BP_BaseObject.BP_BaseObject_C|GetAttachedObjects _asbp_base_object_2) (Variables|Default|GetFirstObject)))
                (:then_3
                  ;[1 1 1] Clear the objects used
                  (Variables|Default|SetFirstObject 0)
                  (Variables|Default|SetSecondObject 0)))
              (else
                (bind _output_get_2 (Variables|Default|SetFirstObject (.hitactor _outhit)))
                (Variables|Default|SetPickedFirst true)))))))))

(fn ConstructionScript
  (|CallParentFunction))