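; BP_Scale is a tool that resizes the physics object the player is aiming at.
; When fired, its multicast event traces from the pawn's camera along the view direction for PhysicsBody objects.
; On a hit, it plays the shoot sound, sets the hit component's world scale to the supplied Scale, and sets mass scale to the product of that vector's axes.
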(event EventMulticastFireWeapon
  (params (OwningPawn :type BP%20Sandbox%20Character%20Object%20Reference) (Pressed :type Boolean) (Scale :type Vector :default "0, 0, 0") (ConstraintInfo :type ST%20Constraint%20Info%20Structure) (Mass%28kg%29 :type Float%20%28single-precision%29) (Thrust%28N%29 :type Float%20%28single-precision%29) (SelectedKey :type Input%20Chord%20Structure))
  (bind (_x _y _z) (Math|Vector|BreakVector Scale))
  (bind _camera (Variables|/Game/Blueprints/BP_SandboxCharacter.BP_SandboxCharacter_C|GetCamera OwningPawn))
  (bind _returnvalue (Transformation|GetWorldLocation _camera))
  (if Pressed
    ;[1 1 1] Trace a line from player's eyes to 1000 cm away
    (bind (_outhit _returnvalue_2) (Collision|LineTraceForObjects _returnvalue (+ _returnvalue (* (Math|Vector|GetForwardVector _camera) 1e+04)) (Utilities|Array|MakeArray "ObjectTypeQuery4") false 0 "None"))
    ;[1 1 1] Check if hit something
    (if _returnvalue_2
      ;[1 1 1] Scale the component!
      (Audio|PlaySoundatLocation "/Game/Audio/SC_ToolShoot.SC_ToolShoot" (Transformation|GetActorLocation OwningPawn) "0, 0, 0" 1.0 1.0 0.0 0 0 0)
      (Transformation|SetWorldScale3D (.hitcomponent _outhit) Scale)
      (Class|PrimitiveComponent|SetMassScale (.hitcomponent _outhit) "None" (* _x _y _z)))))

(fn ConstructionScript
  (|CallParentFunction))