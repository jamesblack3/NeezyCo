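; BP_Mover is a physgun-style tool weapon that grabs, moves, rotates and freezes objects.
; Fire traces from the camera, attaching a physics body with simulation off until release; alt fire freezes the held or aimed-at component.
; Next-weapon axis input changes hold distance, while Use locks look and turns look input into camera-relative rotation.
; Multicast events drive everything, with a gated weapon tick interpolating rotation, grid-snapped while sprint is held.
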(event EventMulticastNextWeapon
  (params (OwningPawn :type BP%20Sandbox%20Character%20Object%20Reference) (AxisValue :type Float%20%28single-precision%29))
  (bind _heldcomponent (Variables|Default|GetHeldComponent))
  ;[1 1 1] Increase or decrease the grab distance with the mouse wheel
  (Utilities|IsValid _heldcomponent
    (:Is%20Valid
      (Transformation|AddWorldOffset (Variables|Default|GetHeldComponent) (* (Math|Vector|Normalize (- (Transformation|GetWorldLocation _heldcomponent) (Transformation|GetWorldLocation (Variables|/Game/Blueprints/BP_SandboxCharacter.BP_SandboxCharacter_C|GetCamera OwningPawn)))) (* AxisValue 5e+01)) false false))))

(event EventMulticastUse
  (params (OwningPawn :type BP%20Sandbox%20Character%20Object%20Reference) (Pressed :type Boolean) (RotationSnap :type Vector :default "0, 0, 0"))
  (bind (_x _y _z) (Math|Vector|BreakVector RotationSnap))
  (bind _heldcomponent (Variables|Default|GetHeldComponent))
  (bind _heldcomponent_2 (Variables|Default|GetHeldComponent))
  ;[1 1 1] Check if holding something
  (Utilities|IsValid (Variables|Default|GetHeldComponent)
    (:Is%20Valid
      ;[1 1 1] Check if pressed
      (if Pressed
        ;[1 1 1] disable looking around so as to focus on the object being rotated
        (Variables|/Game/Blueprints/BP_SandboxCharacter.BP_SandboxCharacter_C|SetLockLook OwningPawn true)
        (Utilities|FlowControl|Gate true) ; enters at Open
        (else
          ;[1 1 1] enable looking around again
          (Variables|/Game/Blueprints/BP_SandboxCharacter.BP_SandboxCharacter_C|SetLockLook OwningPawn false :!label _label)
          (Utilities|FlowControl|Gate true) ; enters at Close
        )))
    (:Is%20Not%20Valid
      (goto _label))))

(event EventMulticastWeaponTick
  (params (OwningPawn :type BP%20Sandbox%20Character%20Object%20Reference) (DeltaTime :type Float%20%28single-precision%29))
  (bind _heldcomponent (Variables|Default|GetHeldComponent))
  (bind _heldcomponent_2 (Variables|Default|GetHeldComponent))
  (bind _heldcomponent_3 (Variables|Default|GetHeldComponent))
  (bind _heldcomponent_4 (Variables|Default|GetHeldComponent))
  ;[1 1 1] Gives the weapon a replicated tick
  (Utilities|IsValid _heldcomponent_4
    (:Is%20Valid
      ;[1 1 1] Snap rotation if shift is held but not E
      (if (stale EventMulticastUse Pressed)
        _
        (elif (Variables|Default|GetSnapRotation)
          (Transformation|SetWorldRotation _heldcomponent_2 (Math|Interpolation|RInterpTo (Transformation|GetWorldRotation _heldcomponent_2) (Math|Rotator|MakeRotator (Math|Float|SnapToGrid(Float) (.roll (Variables|Default|GetHeldRotation)) (.X (Math|Vector|BreakVector (stale EventMulticastUse RotationSnap)))) (Math|Float|SnapToGrid(Float) (.pitch (Variables|Default|GetHeldRotation)) (.Y (Math|Vector|BreakVector (stale EventMulticastUse RotationSnap)))) (Math|Float|SnapToGrid(Float) (.yaw (Variables|Default|GetHeldRotation)) (.Z (Math|Vector|BreakVector (stale EventMulticastUse RotationSnap))))) DeltaTime 1e+01) false false)
          (else
            (Transformation|SetWorldRotation (Variables|Default|GetHeldComponent) (Math|Interpolation|RInterpTo (Transformation|GetWorldRotation _heldcomponent_4) (Variables|Default|GetHeldRotation) DeltaTime 1e+01) false false))))
      (Utilities|FlowControl|Gate true
        (:Exit
          (Utilities|IsValid (Variables|Default|GetHeldComponent)
            (:Is%20Valid
              ;[1 1 1] Rotate!
              (bind _output_get (Variables|Default|SetHeldRotation (Math|Rotator|CombineRotators (Variables|Default|GetHeldRotation) (Math|Rotator|CombineRotators (Math|Vector|RotatorfromAxisandAngle (Math|Vector|GetRightVector (Variables|/Game/Blueprints/BP_SandboxCharacter.BP_SandboxCharacter_C|GetCamera (stale EventMulticastUse OwningPawn))) (Variables|/Game/Blueprints/BP_SandboxCharacter.BP_SandboxCharacter_C|GetLookUp (stale EventMulticastUse OwningPawn))) (Math|Vector|RotatorfromAxisandAngle (Math|Vector|GetUpVector (Variables|/Game/Blueprints/BP_SandboxCharacter.BP_SandboxCharacter_C|GetCamera (stale EventMulticastUse OwningPawn))) (* (Variables|/Game/Blueprints/BP_SandboxCharacter.BP_SandboxCharacter_C|GetLookRight (stale EventMulticastUse OwningPawn)) -1.0))))))
              (if (Variables|Default|GetSnapRotation)
                (Transformation|SetWorldRotation _heldcomponent (Math|Interpolation|RInterpTo (Transformation|GetWorldRotation _heldcomponent) (Math|Rotator|MakeRotator (Math|Float|SnapToGrid(Float) (.Roll (Math|Rotator|BreakRotator _output_get)) (.X (Math|Vector|BreakVector (stale EventMulticastUse RotationSnap)))) (Math|Float|SnapToGrid(Float) (.Pitch (Math|Rotator|BreakRotator _output_get)) (.Y (Math|Vector|BreakVector (stale EventMulticastUse RotationSnap)))) (Math|Float|SnapToGrid(Float) (.Yaw (Math|Rotator|BreakRotator _output_get)) (.Z (Math|Vector|BreakVector (stale EventMulticastUse RotationSnap))))) DeltaTime 1e+01) false false)
                (else
                  (Transformation|SetWorldRotation _heldcomponent_3 (Math|Interpolation|RInterpTo (Transformation|GetWorldRotation _heldcomponent_3) _output_get DeltaTime 1e+01) false false))))))))))

(event EventMulticastSprint
  (params (Pressed :type Boolean))
  (Variables|Default|SetSnapRotation Pressed))

(event EventMulticastFireWeapon
  (params (OwningPawn :type BP%20Sandbox%20Character%20Object%20Reference) (Pressed :type Boolean) (Scale :type Vector :default "0, 0, 0") (ConstraintInfo :type ST%20Constraint%20Info%20Structure) (Mass%28kg%29 :type Float%20%28single-precision%29) (Thrust%28N%29 :type Float%20%28single-precision%29) (SelectedKey :type Input%20Chord%20Structure))
  (bind _camera (Variables|/Game/Blueprints/BP_SandboxCharacter.BP_SandboxCharacter_C|GetCamera OwningPawn))
  (bind _returnvalue (Transformation|GetWorldLocation _camera))
  ;[0.651 1 0.6091] Firing and alt firing
  (Utilities|IsValid OwningPawn
    (:Is%20Valid
      ;;[1 1 1] Check if firing
      (if Pressed
        ;;[1 1 1] Trace a line from player's eyes to 1000 cm away
        (bind (_outhit _returnvalue_2) (Collision|LineTraceForObjects _returnvalue (+ _returnvalue (* (Math|Vector|GetForwardVector _camera) 1e+04)) (Utilities|Array|MakeArray "ObjectTypeQuery4") false 0 "None"))
        ;;[1 1 1] Check if hit something
        (if _returnvalue_2
          ;;[1 1 1] Set the held component and disable physics
          (Physics|SetSimulatePhysics (.hitcomponent _outhit) false)
          (Transformation|AttachComponentToComponent (.hitcomponent _outhit) _camera "None" "KeepWorld" "KeepWorld" "KeepWorld" true)
          (Variables|Default|SetHeldComponent (.hitcomponent _outhit))
          (Variables|Default|SetHeldRotation (Transformation|GetWorldRotation (.hitcomponent _outhit))))
        (else
          ;;[1 1 1] Check if holding an object
          (Utilities|IsValid (Variables|Default|GetHeldComponent)
            (:Is%20Valid
              ;;[1 1 1] release object if holding one
              (Transformation|DetachFromComponent (.hitcomponent _outhit) "KeepWorld" "KeepWorld" "KeepWorld" true)
              (Physics|SetSimulatePhysics (.hitcomponent _outhit) true)
              (Variables|Default|SetHeldComponent 0)
              (Variables|Default|SetHeldRotation "0, 0, 0"))))))))

(event EventMulticastAltFireWeapon
  (params (OwningPawn :type BP%20Sandbox%20Character%20Object%20Reference) (Pressed :type Boolean))
  (bind _camera (Variables|/Game/Blueprints/BP_SandboxCharacter.BP_SandboxCharacter_C|GetCamera OwningPawn))
  (bind _returnvalue (Transformation|GetWorldLocation _camera))
  ;[0.651 1 0.6091] Firing and alt firing
  ;;[1 1 1] Trace a line from player's eyes to 1000 cm away
  (Utilities|IsValid (Variables|Default|GetHeldComponent)
    (:Is%20Valid
      ;;[1 1 1] clear the held component and freeze the object
      (Transformation|DetachFromActor (Components|GetOwner (Variables|Default|GetHeldComponent)) "KeepWorld" "KeepWorld" "KeepWorld")
      (Physics|SetSimulatePhysics (Variables|Default|GetHeldComponent) false)
      (Variables|Default|SetHeldComponent 0)
      (Variables|Default|SetHeldRotation "0, 0, 0"))
    (:Is%20Not%20Valid
      (bind (_outhit _returnvalue_2) (Collision|LineTraceByChannel _returnvalue (+ _returnvalue (* (Math|Vector|GetForwardVector _camera) 1e+04)) "TraceTypeQuery1" false 0 "None"))
      ;;[1 1 1] Check if hit something
      (if _returnvalue_2
        (Utilities|IsValid (Actor|GetAttachParentActor (.hitactor _outhit))
          (:Is%20Valid
            ;;[1 1 1] clear the held component and freeze the object
            (Transformation|DetachFromActor (.hitactor _outhit) "KeepWorld" "KeepWorld" "KeepWorld"))
          (:Is%20Not%20Valid
            _))
        (Physics|SetSimulatePhysics (.hitcomponent _outhit) false)
        (Variables|Default|SetHeldComponent 0)
        (Variables|Default|SetHeldRotation "0, 0, 0")))))

(fn ConstructionScript
  (|CallParentFunction))