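; Player controller for a sandbox that owns the QMenu widget, a toggleable spawn menu.
; BeginPlay creates the menu and adds it to the viewport once.
; The QMenu input action drives a FlipFlop that alternates between showing the menu with cursor and Game-and-UI input, and hiding it with game-only input and viewport focus restored.
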(event EventBeginPlay
  ;[1 1 1] Create QMenu
  (bind _returnvalue (UserInterface|CreateWidget "/Game/Widgets/W_QMenu.W_QMenu_C"))
  (bind _output_get (Variables|Default|SetQMenu _returnvalue))
  (UserInterface|Viewport|AddtoViewport _output_get 1))

(event Input|ActionEvents|InputActionQMenu
  (params (Key :type Key%20Structure))
  ;[1 1 1] Toggle the spawn menu visibility
  (:Pressed
    (Utilities|FlowControl|FlipFlop
      (:A
        (Widget|SetVisibility (Variables|Default|GetQMenu) "Visible")
        (Variables|Default|SetbShowMouseCursor true)
        (Input|SetInputModeGameandUI self (Variables|Default|GetQMenu) "LockAlways" false))
      (:B
        (Widget|SetVisibility (Variables|Default|GetQMenu) "Hidden")
        (Variables|Default|SetbShowMouseCursor false)
        (Input|SetInputModeGameOnly self)
        (Class|WidgetBlueprintLibrary|SetFocustoGameViewport)))))

(fn ConstructionScript)